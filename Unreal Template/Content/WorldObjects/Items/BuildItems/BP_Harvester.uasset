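; BP_Harvester is a buildable harvester item whose logic appears to be an early test stub.
; A DispatchTest event runs through a pass-through macro, MacroTest, and calls GenerateGems with dirt quality and current water pressure.
; Despite its name, GenerateGems only stores the sum of those inputs and hides the static mesh when the item is not paid for.
; The construction script just calls the parent.
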(event `DispatchTest_Event`
  (bind _newparam2 (`self.MacroTest` (`self.NewVar_1`))
    (:`NewParam4`
      (`self.GenerateGems` (`self.DirtQuality`) (`self.Current Water Pressure`))
      (if _newparam2
        _))))

(fn `GenerateGems`
  (params (ThisVariable :type Integer) (ThatVariable :type Integer))
  (set `self.NewVar_0_0` (+ ThisVariable ThatVariable))
  (if (not (`self.PaidFor?`))
    (`SceneComponent.SetVisibility` (`self.StaticMesh`) false false)))

(fn `UserConstructionScript`
  (`parent.UserConstructionScript`))